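; Player combat component for BP_ThirdPersonCharacter, handling target lock, dodge rolls and sword combos.
; Lock-on sphere-traces from the camera for a pawn, attaches a marker actor and steers control rotation toward it each tick.
; Locking switches the character to controller-facing rotation, which lets rolls pick a WASD-based dodge montage.
; Attacks step through montages with a retriggerable combo reset, while a timer-looped sphere trace applies damage, throttled by a DoOnce.
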(event `self.ReceiveBeginPlay`
  ;[0.15 0.1113 0 0.5] Character Ref
  (bind _asbp_third_person_character (cast `/Game/ThirdPerson/Blueprints/BP_ThirdPersonCharacter` (`self.GetOwner`)))
  (set `self.Player BP` _asbp_third_person_character))

(event `EnhancedInput|/Game/ThirdPerson/Input/Actions/IA_Lock`
  (params (ActionValue :type Boolean) (ElapsedSeconds :type "Float (double-precision)") (TriggeredSeconds :type "Float (double-precision)") (InputAction :type "InputAction Object Reference" :default "/Game/ThirdPerson/Input/Actions/IA_Lock.IA_Lock"))
  (bind _returnvalue (`Actor.GetTransform` (`self.Target Lock Actor`)))
  (bind _transformcomponent (`PlayerCameraManager.TransformComponent` (`GameplayStatics.GetPlayerCameraManager` 0)))
  (bind _charactermovement (`Character.CharacterMovement` (`self.Player BP`)))
  (bind _charactermovement_2 (`Character.CharacterMovement` (`self.Player BP`)))
  (bind (_returnvalue_x _returnvalue_y _returnvalue_z) (`KismetMathLibrary.BreakVector` (`SceneComponent.K2_GetComponentLocation` _transformcomponent)))
  ;[0.5073 0 0.2028 0.5] Target Lock
  (:`Started`
    (`self.Target Lock Actor`
      (:`then`
        (set `self.Target Lock Actor` null)
        (set `CharacterMovementComponent.bOrientRotationToMovement` true _charactermovement)
        (set `CharacterMovementComponent.bUseControllerDesiredRotation` false _charactermovement)
        (`Actor.K2_DestroyActor` (`self.Target Lock Widget`)))
      (:`else`
        (bind (_outhit _returnvalue_2) (`KismetSystemLibrary.SphereTraceSingleForObjects` :`End` (+ (`KismetMathLibrary.MakeVector` _returnvalue_x _returnvalue_y (+ _returnvalue_z 20.0)) (* (`KismetMathLibrary.GetForwardVector` (`SceneComponent.K2_GetComponentRotation` _transformcomponent)) 1000.0)) :`Radius` 150.0 :`ObjectTypes` (`|MakeArray` "ObjectTypeQuery3" :!type "EObjectTypeQuery Enum") :`DrawDebugType` "ForDuration" :`DrawTime` 2.0))
        (if _returnvalue_2
          (set `self.Target Lock Actor` (`.HitActor` (`GameplayStatics.BreakHitResult` _outhit)))
          (set `CharacterMovementComponent.bOrientRotationToMovement` false _charactermovement_2)
          (set `CharacterMovementComponent.bUseControllerDesiredRotation` true _charactermovement_2)
          (bind _returnvalue_3 (`|SpawnActorFromClass` "/Game/UI/Lock/BP_TargetLockWidget.BP_TargetLockWidget_C" (`KismetMathLibrary.MakeTransform` (`KismetMathLibrary.MakeVector` (.x (.location _returnvalue)) (.y (.location _returnvalue)) (+ (.z (.location _returnvalue)) 20.0)) (.rotation _returnvalue)) "AlwaysSpawn" "MultiplyWithRoot" null null))
          (bind _output_get (set `self.Target Lock Widget` _returnvalue_3))
          (`Actor.K2_AttachToActor` _output_get (`self.Target Lock Actor`) "None" "SnapToTarget" "SnapToTarget" "SnapToTarget" true))))))

(event `self.ReceiveTick`
  (params (DeltaSeconds :type "Float (single-precision)"))
  (bind (_returnvalue_roll _returnvalue_pitch _returnvalue_yaw) (`KismetMathLibrary.BreakRotator` (`KismetMathLibrary.FindLookAtRotation` (`Actor.K2_GetActorLocation` (`self.Player BP`)) (`Actor.K2_GetActorLocation` (`self.Target Lock Actor`)))))
  ;[0.15 0.03066 0 0.5] Target Lock Update
  (`self.Target Lock Actor`
    (:`then`
      (`Controller.SetControlRotation` (`Pawn.GetController` (`self.Player BP`)) (`KismetMathLibrary.MakeRotator` _returnvalue_roll (+ _returnvalue_pitch -20.0) _returnvalue_yaw)))
    (:`else`)))

(event `EnhancedInput|/Game/ThirdPerson/Input/Actions/IA_Roll`
  (params (ActionValue :type Boolean) (ElapsedSeconds :type "Float (double-precision)") (TriggeredSeconds :type "Float (double-precision)") (InputAction :type "InputAction Object Reference" :default "/Game/ThirdPerson/Input/Actions/IA_Roll.IA_Roll"))
  ;[0.04588 0 0.15 0.5] Make Character Roll
  (:`Started`
    (if (not (`self.Is Rolling?`))
      (set `self.Is Rolling?` true)
      (`|ExecutionSequence`
        (:`then_0`
          (if (`CharacterMovementComponent.bUseControllerDesiredRotation` (`Character.CharacterMovement` (`self.Player BP`)))
            (switch `string` (`KismetTextLibrary.Conv_TextToString` (`KismetInputLibrary.Key_GetDisplayName` (`/Game/ThirdPerson/Blueprints/BP_ThirdPersonCharacter.Direction Key` (`self.Player BP`))))
              (:`W`
                (set `self.MovementDirection` "NewEnumerator0"))
              (:`A`
                (set `self.MovementDirection` "NewEnumerator1"))
              (:`S`
                (set `self.MovementDirection` "NewEnumerator2"))
              (:`D`
                (set `self.MovementDirection` "NewEnumerator3")))))
        (:`then_1`
          (`|PlayMontage` (`Character.Mesh` (`self.Player BP`)) (select `/Game/ThirdPerson/Input/E_MovementDirection` (`self.MovementDirection`) :`NewEnumerator0` "/Game/Animations/Combat/Dodge_F_Montage.Dodge_F_Montage" :`NewEnumerator1` "/Game/Animations/Combat/Dodge_L_Montage.Dodge_L_Montage" :`NewEnumerator2` "/Game/Animations/Combat/Dodge_B_Montage.Dodge_B_Montage" :`NewEnumerator3` "/Game/Animations/Combat/Dodge_R_Montage.Dodge_R_Montage" :!type "AnimMontage Object Reference") 0.7
            (:`OnCompleted`
              _)
            (:`OnInterrupted`
              _))
          (set `self.Is Rolling?` false))))))

(event `EnhancedInput|/Game/ThirdPerson/Input/Actions/IA_Attack`
  (params (ActionValue :type Boolean) (ElapsedSeconds :type "Float (double-precision)") (TriggeredSeconds :type "Float (double-precision)") (InputAction :type "InputAction Object Reference" :default "/Game/ThirdPerson/Input/Actions/IA_Attack.IA_Attack"))
  ;[0.07898 0.15 0.06459 0.5] Input for attack
  (:`Started`
    (set `self.Movement` true)
    (bind _newparam (`self.DoCombo`))
    (`Character.PlayAnimMontage` (`self.Player BP`) _newparam 1.0 "None")))

(event `Do Attack`
  ;[0.1824 0.3636 0.6198 0.5] Do the Attack
  (`/Engine/EditorBlueprintResources/StandardMacros.IncrementInt` (`self.Attack Combo`)
    (:`  `
      (`KismetSystemLibrary.RetriggerableDelay` 2.0)
      (set `self.Attack Combo` 0 :!label _label))))

(event `Reset Combo`
  ;[0.1824 0.3636 0.6198 0.5] Do the Attack
  (goto _label))

(event `End Damage Trace`
  ;[1 0 0.8028 0.5] Create the linetrace of the attack
  (if (`KismetSystemLibrary.K2_IsValidTimerHandle` (stale `Beging Damage Trace` _returnvalue))
    (`KismetSystemLibrary.K2_ClearAndInvalidateTimerHandle` (stale `Beging Damage Trace` _returnvalue))))

(event `Beging Damage Trace`
  ;[1 0 0.8028 0.5] Create the linetrace of the attack
  (bind _returnvalue (`KismetSystemLibrary.K2_SetTimerDelegate` (delegate `Damage Trace`) 0.01 true)))

(event `Damage Trace`
  (bind _player_bp (`self.Player BP`))
  ;[1 0 0.8028 0.5] Create the linetrace of the attack
  (bind (_outhit _returnvalue) (`KismetSystemLibrary.SphereTraceSingle` :`Start` (`SceneComponent.K2_GetComponentLocation` (`/Game/ThirdPerson/Blueprints/BP_ThirdPersonCharacter.Start Trace` _player_bp)) :`End` (`SceneComponent.K2_GetComponentLocation` (`/Game/ThirdPerson/Blueprints/BP_ThirdPersonCharacter.End Trace` _player_bp)) :`Radius` 25.0 :`TraceChannel` "TraceTypeQuery1" :`DrawDebugType` "ForOneFrame"))
  (if _returnvalue
    (`/Engine/EditorBlueprintResources/StandardMacros.DoOnce` false :!label _label_2
      (:`Completed`
        (`GameplayStatics.ApplyDamage` (`.HitActor` (`GameplayStatics.BreakHitResult` _outhit)) (`self.Sword Damage`))
        (`KismetSystemLibrary.Delay` 0.3)
        (goto _label_2 :!via `Reset`)))))

(fn `DoCombo`
  (returns (NewParam :type "AnimMontage Object Reference"))
  (bind _attack (`self.Attack`))
  (if (>= (`self.Attack Combo`) (- (`KismetArrayLibrary.Array_Length` (`self.Attack`)) 1))
    (`self.Reset Combo`)
    (return (`|GetArrayItem` _attack (`KismetArrayLibrary.Array_LastIndex` _attack)))
    (else
      (`self.Do Attack`)
      (return (`|GetArrayItem` (`self.Attack`) (- (`self.Attack Combo`) 1))))))