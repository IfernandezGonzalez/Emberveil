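; BP_Enemy is an enemy character with a sword attack montage, a health bar widget and ragdoll death.
; Begin/EndSwordTrace start and stop a looping timer that sphere-traces between two points, applying sword damage through a DoOnce gate with a short cooldown.
; Incoming damage lowers a BPCStats value, and that component receives the widget's health bar on BeginPlay.
; Die disables movement, enables mesh physics and destroys the actor after a delay.
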(event `/Game/Combat/BPI_Damage.End Sword Trace`
  ;[0.15 0.02078 0.02078 0.5] Create the linetrace of the attack
  (if (`KismetSystemLibrary.K2_IsValidTimerHandle` (stale `/Game/Combat/BPI_Damage.Begin Sword Trace` _returnvalue))
    (`KismetSystemLibrary.K2_ClearAndInvalidateTimerHandle` (stale `/Game/Combat/BPI_Damage.Begin Sword Trace` _returnvalue))))

(event `/Game/Combat/BPI_Damage.Begin Sword Trace`
  ;[0.15 0.02078 0.02078 0.5] Create the linetrace of the attack
  (bind _returnvalue (`KismetSystemLibrary.K2_SetTimerDelegate` (delegate `Damage Trace`) 0.01 true)))

(event `Damage Trace`
  ;[0.15 0.02078 0.02078 0.5] Create the linetrace of the attack
  (if (not (`self.IsDead?`))
    (bind (_outhit _returnvalue) (`KismetSystemLibrary.SphereTraceSingle` :`Start` (`SceneComponent.K2_GetComponentLocation` (`self.Start`)) :`End` (`SceneComponent.K2_GetComponentLocation` (`self.End`)) :`Radius` 25.0 :`TraceChannel` "TraceTypeQuery1" :`DrawDebugType` "ForOneFrame"))
    (if _returnvalue
      (`/Engine/EditorBlueprintResources/StandardMacros.DoOnce` false :!label _label
        (:`Completed`
          (`GameplayStatics.ApplyDamage` (`.HitActor` (`GameplayStatics.BreakHitResult` _outhit)) (`self.Sword Damage`) null self)
          (`KismetSystemLibrary.Delay` 0.3)
          (goto _label :!via `Reset`))))))

(event `/Game/Combat/BPI_Damage.Die`
  ;[0.5406 0 0.4237 0.5] Enemy Die
  (`CharacterMovementComponent.DisableMovement` (`self.CharacterMovement`))
  (`PrimitiveComponent.SetSimulatePhysics` (`self.Mesh`) true)
  (set `self.IsDead?` true)
  (`KismetSystemLibrary.Delay` 5.0)
  (`self.K2_DestroyActor`))

(event `self.ReceiveBeginPlay`
  ;[0.01391 0.15 0.1356 0.5] Set Enemy Health bar
  (bind _asw_enemy_health (cast `/Game/UI/Player/W_EnemyHealth` (`WidgetComponent.GetWidget` (`self.Widget`))))
  (`/Game/Combat/Stats/BPC_Stats.Set Health bar` (`self.BPC_Stats`) (`/Game/UI/Player/W_EnemyHealth.HealthBar` _asw_enemy_health)))

(event `self.ReceiveAnyDamage`
  (params (Damage :type "Float (single-precision)") (DamageType :type "DamageType Object Reference") (InstigatedBy :type "Controller Object Reference") (DamageCauser :type "Actor Object Reference"))
  ;[0.15 0.1472 0 0.5] Apply Damage
  (`/Game/Combat/Stats/BPC_Stats.Increase value` (`self.BPC_Stats`) "NewEnumerator0" (* Damage -1.0)))

(fn `Attack`
  (returns (Duration :type "Float (double-precision)"))
  (bind _returnvalue (`self.PlayAnimMontage` "/Game/ROG_Creatures/Stickman/Animations/AM_Stickman_Attack_01.AM_Stickman_Attack_01"))
  (return _returnvalue))

(fn `UserConstructionScript`)